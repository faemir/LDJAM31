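; Behavior tree task that sends an AI Seeker to a random item spawn point.
; On execute it caches the SeekerController, picks a random ItemSpawnPoint actor and opens a Gate.
; While the Seeker is alive, Tick passes through that Gate to call AIMoveTo, which finishes the task and closes the Gate on success or failure.
; A failed controller cast only prints a message, without finishing the task.
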(event `self.ReceiveTick`
  (params (OwnerActor :type "Actor Object Reference") (DeltaSeconds :type "Float (single-precision)"))
  (bind _returnvalue (`Controller.K2_GetPawn` (`self.controllerRef`)))
  (bind _asseeker (cast `/Game/Blueprints/Seeker/Seeker` _returnvalue))
  (if (`/Game/Blueprints/Seeker/Seeker.isAlive` _asseeker)
    (`/Engine/EditorBlueprintResources/StandardMacros.Gate` true :!label _label
      (:`Exit`
        (`|AIMoveTo` _returnvalue (0.0 0.0 0.0) (`self.randomActor`) 500.0
          (:`OnSuccess`
            (`self.FinishExecute` true)
            (goto _label :!via `Close`))
          (:`OnFail`
            (`self.FinishExecute` false)
            (goto _label :!via `Close`)))))))

(event `self.ReceiveExecute`
  (params (OwnerActor :type "Actor Object Reference"))
  (bind _asseeker_controller (cast `/Game/Blueprints/Seeker/SeekerController` OwnerActor)
    (:`then`
      (set `self.controllerRef` _asseeker_controller)
      (bind _outactors (`GameplayStatics.GetAllActorsOfClass` "/Game/Blueprints/itemSpawnPoint.itemSpawnPoint_C"))
      (set `self.randomActor` (`KismetArrayLibrary.Array_Get` _outactors (`KismetMathLibrary.RandomIntegerInRange` 0 (- (`KismetArrayLibrary.Array_Length` _outactors) 1))))
      (goto _label :!via `Open`))
    (:`CastFailed`
      (`KismetSystemLibrary.PrintString` "Cast failed in MoveToRandomSpawnPoint" true true (struct :`R` 1.0 :`B` 0.068705 :`A` 1.0)))))