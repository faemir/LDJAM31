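; Behavior tree tick logic that decides when a Seeker AI aggros onto the player.
; Each tick it clears the TargetToFollow blackboard key, then line traces on the Camera channel from the controlled pawn to the player, ignoring itself.
; If the trace hits a MyCharacter within 1000 units, that actor becomes TargetToFollow, so losing sight or range drops the target.
; The trace leaves debug drawing enabled.
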(event `self.ReceiveTick`
  (params (OwnerActor :type "Actor Object Reference") (DeltaSeconds :type "Float (single-precision)"))
  (bind _asseeker_controller (cast `/Game/Blueprints/Seeker/SeekerController` OwnerActor)
    (:`then`
      (set `self.controllerRef` _asseeker_controller)
      (bind _returnvalue (`Controller.K2_GetPawn` _asseeker_controller))
      (set `self.myLocation` (`Actor.K2_GetActorLocation` _returnvalue))
      (set `self.actorRef` _returnvalue)
      (`BTFunctionLibrary.SetBlackboardValueAsObject` (`self.targetToFollow`))
      (bind _outhit (`KismetSystemLibrary.LineTraceSingle` (`self.myLocation`) (`Actor.K2_GetActorLocation` (`GameplayStatics.GetPlayerPawn` 0)) "TraceTypeQuery2" false (`|MakeArray` (`self.actorRef`)) "ForDuration"))
      (bind (_bblockinghit _time _location _normal _impactpoint _impactnormal _physmat _hitactor) (`GameplayStatics.BreakHitResult` _outhit))
      (cast `/Game/Blueprints/MyCharacter` _hitactor)
      (if (< (`KismetMathLibrary.VSize` (- (`self.myLocation`) _location)) 1000.0)
        (`BTFunctionLibrary.SetBlackboardValueAsObject` (`self.targetToFollow`) _hitactor)))
    (:`CastFailed`
      (`KismetSystemLibrary.PrintString` "Cast failed in SnowmanAgro" true true (struct :`R` 1.0 :`G` 0.023868 :`A` 1.0)))))