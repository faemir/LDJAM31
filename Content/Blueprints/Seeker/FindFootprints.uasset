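; Behavior tree node that finds the freshest footprint breadcrumb near the Seeker's pawn.
; Each tick it clears the Footprint blackboard key and runs a multi-sphere object trace around the pawn for footstep object types.
; A helper seeds the candidate with the first breadcrumb hit, then a loop keeps the latest TimePlaced and writes it to the Footprint key.
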(event `self.ReceiveTick`
  (params (OwnerActor :type "Actor Object Reference") (DeltaSeconds :type "Float (single-precision)"))
  (bind _mylocation (`self.myLocation`))
  (bind _abreadcrumb (`self.aBreadcrumb`))
  (bind _asseeker_controller (cast `/Game/Blueprints/Seeker/SeekerController` OwnerActor)
    (:`then`
      (set `self.controllerRef` _asseeker_controller)
      (bind _returnvalue (`Controller.K2_GetPawn` _asseeker_controller))
      (set `self.myLocation` (`Actor.K2_GetActorLocation` _returnvalue))
      (set `self.actorRef` _returnvalue)
      (`BTFunctionLibrary.SetBlackboardValueAsObject` (`self.footprint`))
      (bind _outhits (`KismetSystemLibrary.SphereTraceMultiForObjects` :`Start` _mylocation :`End` (+ _mylocation (0.0 0.0 10.0)) :`Radius` 350.0 :`ObjectTypes` (`self.footstepTypes`) :`DrawDebugType` "ForOneFrame"))
      (for _array_element _outhits
        (bind _asbreadcrumb (cast `/Game/Blueprints/Breadcrumb` (`.HitActor` (`GameplayStatics.BreakHitResult` _array_element)))
          (:`then`
            (set `self.freshestBreadcrumb` _asbreadcrumb)
            (break))
          (:`CastFailed`
            (set `self.freshestBreadcrumb` null))))
      (if (`KismetSystemLibrary.IsValid` (`self.freshestBreadcrumb`))
        (for _array_element_2 _outhits
          (bind _asbreadcrumb_2 (cast `/Game/Blueprints/Breadcrumb` (`.HitActor` (`GameplayStatics.BreakHitResult` _array_element_2))))
          (set `self.aBreadcrumb` _asbreadcrumb_2)
          (if (< (`/Game/Blueprints/Breadcrumb.timePlaced` (`self.freshestBreadcrumb`)) (`/Game/Blueprints/Breadcrumb.timePlaced` _abreadcrumb))
            (set `self.freshestBreadcrumb` _abreadcrumb)))
        (`BTFunctionLibrary.SetBlackboardValueAsObject` (`self.footprint`) (`self.freshestBreadcrumb`))))
    (:`CastFailed`
      (`KismetSystemLibrary.PrintString` "Cast failed in SnowmanAgro" true true (struct :`R` 1.0 :`G` 0.023868 :`A` 1.0)))))