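; Behavior tree task that moves a Seeker pawn to the actor stored in the TargetObject blackboard key.
; Execution caches the SeekerController and opens a gate, letting Tick reissue AIMoveTo while the Seeker is alive.
; A successful move finishes the task as failed and closes the gate; move failure is not handled.
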(event `self.ReceiveTick`
  (params (OwnerActor :type "Actor Object Reference") (DeltaSeconds :type "Float (single-precision)"))
  (bind _asseeker (cast `/Game/Blueprints/Seeker/Seeker` (`Controller.K2_GetPawn` (`self.controllerRef`))))
  (if (`/Game/Blueprints/Seeker/Seeker.isAlive` _asseeker)
    (`/Engine/EditorBlueprintResources/StandardMacros.Gate` true :!label _label
      (:`Exit`
        (`|AIMoveTo` (`Controller.K2_GetPawn` (`self.controllerRef`)) (0.0 0.0 0.0) (`BTFunctionLibrary.GetBlackboardValueAsActor` (`self.TargetObject`))
          (:`OnSuccess`
            (`self.FinishExecute` false)
            (`self.CloseGate`)))))))

(event `self.ReceiveExecute`
  (params (OwnerActor :type "Actor Object Reference"))
  (bind _asseeker_controller (cast `/Game/Blueprints/Seeker/SeekerController` OwnerActor))
  (set `self.controllerRef` _asseeker_controller)
  (goto _label :!via `Open`))

(event `CloseGate`
  (goto _label :!via `Close`))