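; Item spawner actor that keeps a single ItemPickup present in the level.
; On BeginPlay it starts a looping one-second timer that calls spawnItem.
; Each tick of that timer checks for existing ItemPickup actors and, when none remain, spawns one at the transform of a randomly chosen ItemSpawnPoint.
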(event `self.ReceiveBeginPlay`
  (`KismetSystemLibrary.K2_SetTimer` null "spawnItem" 1.0 true))

(event `spawnItem`
  (bind _outactors (`GameplayStatics.GetAllActorsOfClass` "/Game/Blueprints/itemPickup.itemPickup_C"))
  (if (== (`KismetArrayLibrary.Array_Length` _outactors) 0)
    (bind _outactors_2 (`GameplayStatics.GetAllActorsOfClass` "/Game/Blueprints/itemSpawnPoint.itemSpawnPoint_C"))
    (`|SpawnActorFromClass` "/Game/Blueprints/itemPickup.itemPickup_C" (`self.GetTransform` (`KismetArrayLibrary.Array_Get` _outactors_2 (`KismetMathLibrary.RandomIntegerInRange` 0 (- (`KismetArrayLibrary.Array_Length` _outactors_2) 1)))))))

(fn `UserConstructionScript`)