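; Player start actor that spawns and possesses the player character and puts up the score HUD when play begins.
; On BeginPlay it spawns MyCharacter slightly above its own location, using a fixed rotation rather than its own.
; It then casts the first player controller to MyController to possess the character, creates the Score widget, stores it as GameHUD and adds it to the viewport.
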(event `self.ReceiveBeginPlay`
  (bind _returnvalue (`|SpawnActorFromClass` "/Game/Blueprints/MyCharacter.MyCharacter_C" (`KismetMathLibrary.MakeTransform` (`KismetMathLibrary.MakeVector` (.x (.location (`self.GetTransform`))) (.y (.location (`self.GetTransform`))) (+ (.z (.location (`self.GetTransform`))) 100.0)) (struct :`Pitch` 1.0 :`Yaw` 1.0 :`Roll` 1.0) (1.0 1.0 1.0))))
  (bind _asmy_controller (cast `/Game/Blueprints/MyController` (`GameplayStatics.GetPlayerController` 0)))
  (`Controller.Possess` _asmy_controller _returnvalue)
  (bind _returnvalue_2 (`|CreateWidget` "/Game/Blueprints/score.score_C"))
  (set `self.gameHUD` _returnvalue_2)
  (`UserWidget.AddToViewport` _returnvalue_2))

(fn `UserConstructionScript`)