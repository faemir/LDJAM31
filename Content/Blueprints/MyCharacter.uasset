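; Player character Blueprint with a dash attack against AI snowman enemies and game over on enemy contact.
; Dash start and stop events toggle a flag and switch between normal and boosted walk speed.
; While dashing, Tick runs a multi sphere trace around the character and calls SnowmanDie on AI characters hit.
; Hitting a living AI character records latest and highest scores through MyGame, then opens the game over map.
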(event `DashStart`
  (set `CharacterMovementComponent.MaxWalkSpeed` 1200.0 (`self.CharacterMovement`))
  (set `self.dashing` true))

(event `DashStop`
  (set `CharacterMovementComponent.MaxWalkSpeed` 600.0 (`self.CharacterMovement`))
  (set `self.dashing` false))

(event `self.ReceiveHit`
  (params (MyComp :type "PrimitiveComponent Object Reference") (Other :type "Actor Object Reference") (OtherComp :type "PrimitiveComponent Object Reference") (bSelfMoved :type Boolean) (HitLocation :type "Object.Vector Structure") (HitNormal :type "Object.Vector Structure") (NormalImpulse :type "Object.Vector Structure") (Hit :type "EngineTypes.HitResult Structure (by ref)"))
  ;[1 1 1] when enemy touches, die and load game over screen
  (if (== (`GameplayStatics.GetObjectClass` Other) "/Game/Blueprints/AI_Character/AI_Character.AI_Character_C")
    (bind _asai_character (cast `/Game/Blueprints/AI_Character/AI_Character` Other))
    (if (`/Game/Blueprints/AI_Character/AI_Character.isAlive` _asai_character)
      (bind _asmy_game (cast `/Game/Blueprints/MyGame` (`GameplayStatics.GetGameMode`)))
      (`/Game/Blueprints/MyGame.setLatestScore` _asmy_game)
      (`/Game/Blueprints/MyGame.setHighestScore` _asmy_game)
      (`GameplayStatics.OpenLevel` "gameOver_map"))))

(event `self.ReceiveTick`
  (params (DeltaSeconds :type "Float (single-precision)"))
  (bind _returnvalue (`self.K2_GetActorLocation`))
  (if (`self.dashing`)
    (bind _outhits (`KismetSystemLibrary.SphereTraceMultiForObjects` _returnvalue (+ _returnvalue (0.0 0.0 15.0)) 200.0 (`self.DashHitTypes`)))
    (for _array_element _outhits
      (bind (_bblockinghit _time _location _normal _impactpoint _impactnormal _physmat _hitactor) (`GameplayStatics.BreakHitResult` _array_element))
      (bind _asai_character (cast `/Game/Blueprints/AI_Character/AI_Character` _hitactor))
      (`/Game/Blueprints/AI_Character/AI_Character.snowmanDie` _asai_character _location))))

(fn `UserConstructionScript`)