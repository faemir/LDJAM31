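; PlaceBreadcrumbs is a Blueprint that leaves a trail of Breadcrumb actors along the path of the pawn controlled by player 0.
; BeginPlay spawns the first breadcrumb at the pawn's location.
; Each Tick spawns another once the pawn is farther than DistanceBetweenBreadcrumbs from the last one, then stores the new actor's location as the next reference point.
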(event `self.ReceiveTick`
  (params (DeltaSeconds :type "Float (single-precision)"))
  (bind _returnvalue (`self.K2_GetActorLocation` (`Controller.K2_GetPawn` (`GameplayStatics.GetPlayerController` 0))))
  (if (> (`KismetMathLibrary.VSize` (- _returnvalue (`self.LastBreadcrumbLocation`))) (`self.DistanceBetweenBreadcrumbs`))
    (bind _returnvalue_2 (`|SpawnActorFromClass` "/Game/Blueprints/Breadcrumb.Breadcrumb_C" (`KismetMathLibrary.Conv_VectorToTransform` _returnvalue) :!label _label))
    (set `self.LastBreadcrumbLocation` (`self.K2_GetActorLocation` _returnvalue_2))))

(event `self.ReceiveBeginPlay`
  (goto _label))

(fn `UserConstructionScript`)