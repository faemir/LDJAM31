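; Item pickup actor that rewards the player and spawns a new AI character when collected.
; On overlap with MyCharacter, it sets the controller's CanDash from its Special variable and adds score.
; It then loops over all ItemSpawnPoint actors to find the one farthest from the player pawn.
; An AI_Character with a default controller spawns at that point, and the pickup destroys itself.
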(event `self.ReceiveActorBeginOverlap`
  (params (OtherActor :type "Actor Object Reference"))
  (bind _returnvalue (`self.K2_GetActorLocation` (`GameplayStatics.GetPlayerPawn` 0)))
  (if (== (`GameplayStatics.GetObjectClass` OtherActor) "/Game/Blueprints/MyCharacter.MyCharacter_C")
    (bind _asmy_controller (cast `/Game/Blueprints/MyController` (`GameplayStatics.GetPlayerController` 0)))
    (set `/Game/Blueprints/MyController.canDash` (`self.Special`) _asmy_controller)
    (`/Game/Blueprints/MyController.addScore` _asmy_controller 5)
    (bind _outactors (`GameplayStatics.GetAllActorsOfClass` "/Game/Blueprints/itemSpawnPoint.itemSpawnPoint_C"))
    (set `self.FurthestAway` (`KismetArrayLibrary.Array_Get` _outactors))
    (for _array_element _outactors
      (if (> (`KismetMathLibrary.VSize` (- (`self.K2_GetActorLocation` _array_element) _returnvalue)) (`KismetMathLibrary.VSize` (- (`self.K2_GetActorLocation` (`self.FurthestAway`)) _returnvalue)))
        (set `self.FurthestAway` _array_element)))
    (bind _returnvalue_2 (`|SpawnActorFromClass` "/Game/Blueprints/AI_Character/AI_Character.AI_Character_C" (`self.GetTransform` (`self.FurthestAway`))))
    (`Pawn.SpawnDefaultController` _returnvalue_2)
    (`self.K2_DestroyActor`)))

(fn `UserConstructionScript`)