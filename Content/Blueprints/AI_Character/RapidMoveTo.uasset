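; Behavior tree task that makes a follower AI character chase the actor stored in the TargetToFollow blackboard key.
; Execution caches the Follower_AI_CON controller and opens a gate, letting Tick repeatedly issue AI MoveTo while the controlled AI_Character is alive.
; A successful move finishes the task as failed and closes the gate; a failed move has no handler, so the requests continue.
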(event `self.ReceiveTick`
  (params (OwnerActor :type "Actor Object Reference") (DeltaSeconds :type "Float (single-precision)"))
  (bind _asai_character (cast `/Game/Blueprints/AI_Character/AI_Character` (`Controller.K2_GetPawn` (`self.AI CON Ref`))))
  (if (`/Game/Blueprints/AI_Character/AI_Character.isAlive` _asai_character)
    (`/Engine/EditorBlueprintResources/StandardMacros.Gate` true :!label _label
      (:`Exit`
        (`|AIMoveTo` (`Controller.K2_GetPawn` (`self.AI CON Ref`)) (0.0 0.0 0.0) (`BTFunctionLibrary.GetBlackboardValueAsActor` (`self.Target to Follow`)) 50.0
          (:`OnSuccess`
            (`self.FinishExecute` false)
            (`self.CloseGate`)))))))

(event `self.ReceiveExecute`
  (params (OwnerActor :type "Actor Object Reference"))
  (bind _asfollower_ai_con (cast `/Game/Blueprints/AI_Character/Follower_AI_CON` OwnerActor))
  (set `self.AI CON Ref` _asfollower_ai_con)
  (goto _label :!via `Open`))

(event `CloseGate`
  (goto _label :!via `Close`))