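; Behavior tree tick logic that picks the follower AI's blackboard target: player, breadcrumb or item spawn point.
; A player within a short radius becomes the target and switches the character to running, otherwise it walks.
; When not chasing, a debug-drawn sphere trace finds nearby breadcrumbs and targets the most recently placed one.
; With no target or trail, it draws randomly from ItemSpawnPoint actors to set target object and location.
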(event `self.ReceiveTick`
  (params (OwnerActor :type "Actor Object Reference") (DeltaSeconds :type "Float (single-precision)"))
  (bind _returnvalue (`GameplayStatics.GetPlayerPawn` 0))
  (bind _a_breadcrumb (`self.A Breadcrumb`))
  (bind _freshest_breadcrumb (`self.Freshest Breadcrumb`))
  (bind _returnvalue_2 (`Actor.K2_GetActorLocation` _returnvalue))
  (bind _asfollower_ai_con (cast `/Game/Blueprints/AI_Character/Follower_AI_CON` OwnerActor))
  (bind _asai_character (cast `/Game/Blueprints/AI_Character/AI_Character` (`Controller.K2_GetPawn` _asfollower_ai_con)))
  (set `self.AI_Character Ref` _asai_character)
  (bind _asfollower_ai_con_2 (cast `/Game/Blueprints/AI_Character/Follower_AI_CON` OwnerActor))
  (set `self.AICON Ref` _asfollower_ai_con_2)
  (bind _returnvalue_3 (`Actor.K2_GetActorLocation` (`Controller.K2_GetPawn` _asfollower_ai_con_2)))
  (set `self.MyLocation` _returnvalue_3)
  (`|ExecutionSequence`
    (:`then_0`
      (set `self.ChasingPlayer` (< (`KismetMathLibrary.VSize` (- _returnvalue_2 _returnvalue_3)) 500.0))
      (if (`self.ChasingPlayer`)
        (`BTFunctionLibrary.SetBlackboardValueAsObject` (`self.Target To Follow`) _returnvalue)
        (`BTFunctionLibrary.SetBlackboardValueAsVector` (`self.Target Location`) _returnvalue_2)
        (`/Game/Blueprints/AI_Character/AI_Character.AIRun` (`self.AI_Character Ref`))
        (else
          (`BTFunctionLibrary.SetBlackboardValueAsObject` (`self.Target To Follow`))
          (`/Game/Blueprints/AI_Character/AI_Character.AIWalk` (`self.AI_Character Ref`)))))
    (:`then_1`
      (if (not (`self.ChasingPlayer`))
        (bind _outhits (`KismetSystemLibrary.SphereTraceMultiForObjects` :`Start` _returnvalue_3 :`End` (+ _returnvalue_3 (0.0 0.0 15.0)) :`Radius` 400.0 :`ObjectTypes` (`self.Breadcrumb Types`) :`DrawDebugType` "ForOneFrame"))
        (for _array_element _outhits
          (bind _asbreadcrumb (cast `/Game/Blueprints/Breadcrumb` (`.HitActor` (`GameplayStatics.BreakHitResult` _array_element)))
            (:`then`
              (set `self.Freshest Breadcrumb` _asbreadcrumb)
              (break))
            (:`CastFailed`
              (set `self.Freshest Breadcrumb` null))))
        (set `self.FollowingCrumbs` (`KismetSystemLibrary.IsValid` (`self.Freshest Breadcrumb`)))
        (if (`self.FollowingCrumbs`)
          (for _array_element_2 _outhits
            (bind _asbreadcrumb_2 (cast `/Game/Blueprints/Breadcrumb` (`.HitActor` (`GameplayStatics.BreakHitResult` _array_element_2))))
            (set `self.A Breadcrumb` _asbreadcrumb_2)
            (if (< (`/Game/Blueprints/Breadcrumb.timePlaced` (`self.Freshest Breadcrumb`)) (`/Game/Blueprints/Breadcrumb.timePlaced` _a_breadcrumb))
              (set `self.Freshest Breadcrumb` _a_breadcrumb)))
          (`BTFunctionLibrary.SetBlackboardValueAsObject` (`self.Target To Follow`) _freshest_breadcrumb)
          (`BTFunctionLibrary.SetBlackboardValueAsVector` (`self.Target Location`) (`Actor.K2_GetActorLocation` _freshest_breadcrumb)))))
    (:`then_2`
      (if (and (not (`KismetSystemLibrary.IsValid` (`BTFunctionLibrary.GetBlackboardValueAsObject` (`self.Target To Follow`)))) (not (`self.FollowingCrumbs`)))
        (bind _outactors (`GameplayStatics.GetAllActorsOfClass` "/Game/Blueprints/itemSpawnPoint.itemSpawnPoint_C"))
        (bind _item (`KismetArrayLibrary.Array_Get` _outactors (`KismetMathLibrary.RandomIntegerInRange` 0 (- (`KismetArrayLibrary.Array_Length` _outactors) 1))))
        (`BTFunctionLibrary.SetBlackboardValueAsObject` (`self.Target To Follow`) _item)
        (`BTFunctionLibrary.SetBlackboardValueAsVector` (`self.Target Location`) (`Actor.K2_GetActorLocation` _item))))))